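; Blueprint Interface for animation Blueprints in a close combat system, declaring the calls that other objects make on a character's animation instance.
; Setters pass in state such as combat, blocking, damage, death, jump, lean, equipment and movement blend space.
; Getters request animations for rolls, avoids, combat transitions, fatalities, skills, taunts, blocks and player damage.
; FE_ functions declare effect hooks for weapon drop, slow motion, damage particles, death and fatalities.
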(fn `ChangeMovementAnimation`
  (params (BlendSpace :type "BlendSpaceBase Object Reference")))

(fn `DamageMelee`
  (params (DamageParameters :type "/Game/Migrate/CloseCombat/Blueprints/Weapon/ParentWeapon/DamageParam_Struct Structure")))

(fn `Equip`
  (params (Equip :type Boolean)))

(fn `FE_DamageParticle`
  (params (Socket :type Name) (Particle :type "ParticleSystem Object Reference")))

(fn `FE_Dead`
  (params (WithSlowMotionEffect :type Boolean) (PhysImpulse :type Boolean)))

(fn `FE_FatalityEffects`
  (params (Victim :type "Actor Object Reference") (Fatality_type :type "/Game/Migrate/CloseCombat/Blueprints/Player/Components/FatalityType_Enum Enum" :default "NewEnumerator0")))

(fn `FE_SlowMotion`
  (params (SlowMotionStrengthm :type "Float (double-precision)") (TimeInSlowMotion :type "Float (double-precision)")))

(fn `FE_WeaponDrop`)

(fn `GetAnim_Avoid`
  (params (Direction :type String))
  (returns (Animation :type "AnimSequence Object Reference"))
  (return null))

(fn `GetAnim_Block`
  (params (Attack :type Boolean) (Index :type Integer) (RandomAnimations :type Boolean))
  (returns (Animation :type "AnimSequence Object Reference"))
  (return null))

(fn `GetAnim_CombatTransition`
  (params (State :type String))
  (returns (Animation :type "AnimSequence Object Reference"))
  (return null))

(fn `GetAnim_Fatality`
  (params (Stealth :type Boolean) (FatalityType :type String))
  (returns (FatalityArray :type "Array of /Game/Migrate/CloseCombat/Blueprints/Player/Components/Fatality_Struct Structure"))
  (return))

(fn `GetAnim_Player_Damage`
  (returns (DamageAnim :type "AnimSequenceBase Object Reference"))
  (return null))

(fn `GetAnim_Roll`
  (params (Direction :type String))
  (returns (Animation :type "AnimSequence Object Reference"))
  (return null))

(fn `GetAnim_Skills`
  (params (SkillName :type String))
  (returns (Animation :type "AnimSequence Object Reference"))
  (return null))

(fn `GetAnim_Taunts`
  (params (Index :type Integer) (RandomTaunt :type Boolean))
  (returns (Animation :type "AnimSequence Object Reference"))
  (return null))

(fn `Set_Armed`
  (params (Armed :type Boolean)))

(fn `Set_Blocking`
  (params (Blocking :type Boolean)))

(fn `Set_Combat`
  (params (Combat :type Boolean)))

(fn `Set_Damage`
  (params (Damage :type Boolean)))

(fn `Set_Dead`
  (params (Dead :type Boolean)))

(fn `Set_Direction_Targeting`
  (params (Direction_Targeting :type "Float (double-precision)")))

(fn `Set_Jump`
  (params (IsJump :type Boolean)))

(fn `Set_Lean`
  (params (Lean :type "Float (double-precision)")))

(fn `Set_ThrowRock`)